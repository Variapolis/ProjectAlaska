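; Sliding airlock door Blueprint with two panels that part in opposite directions and can start open.
; BeginPlay plays the timeline if Open is set, and the Activate event plays or reverses it based on Open.
; Each timeline update lerps both panels' relative locations, flips Open and sets Opening.
; Opening blocks further activation until the timeline finishes.
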(event EventBeginPlay
  ;[1 1 1] Open
  ;;[1 1 1] BeginPlay
  (if (Variables|Default|GetOpen)
    (bind _newtrack_0 (Timeline|Timeline_0 Play)
      (:Update
        (Variables|Default|SetOpen (not (Variables|Default|GetOpen)))
        (Variables|Default|SetOpening true)
        (Transformation|SetRelativeLocation (Variables|Default|GetLeftDoor) (Math|Vector|Lerp(Vector) "0, 0, 0" "0,-100.000000, 0" _newtrack_0) false false)
        (Transformation|SetRelativeLocation (Variables|Default|GetRightDoor) (Math|Vector|Lerp(Vector) "0, 0, 0" "0,100.000000, 0" _newtrack_0) false false))
      (:Finished
        (Variables|Default|SetOpening false)))))

(event EventActivate
  ;[1 1 1] Open
  ;;[1 1 1] Activation
  (if (not (Variables|Default|GetOpening))
    (if (Variables|Default|GetOpen)
      (bind _newtrack_0 (Timeline|Timeline_0 Reverse)
        (:Update
          (Variables|Default|SetOpen (not (Variables|Default|GetOpen)))
          (Variables|Default|SetOpening true)
          (Transformation|SetRelativeLocation (Variables|Default|GetLeftDoor) (Math|Vector|Lerp(Vector) "0, 0, 0" "0,-100.000000, 0" _newtrack_0) false false)
          (Transformation|SetRelativeLocation (Variables|Default|GetRightDoor) (Math|Vector|Lerp(Vector) "0, 0, 0" "0,100.000000, 0" _newtrack_0) false false))
        (:Finished
          (Variables|Default|SetOpening false)))
      (else
        (Timeline|Timeline_0 Play)))))

(fn ConstructionScript)