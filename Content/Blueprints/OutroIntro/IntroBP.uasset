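; IntroBP is an actor that runs the game's intro when play begins.
; It creates and shows IntroWidget, plays its intro, and disables player character movement, restoring Walking mode after a five-second delay.
; In parallel, a SoundControl timeline drives the Master and VolumeSounds class volumes through overrides on MasterSoundMix, pushing the mix on every update.
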(event Custom|SoundFade
  (bind _newtrack_0 (Timeline|SoundControl Play)
    (:Update
      (Audio|SetSoundMixClassOverride "/Game/Sounds/MasterSoundMix.MasterSoundMix" "/Engine/EngineSounds/Master.Master" _newtrack_0 1.0 0.0 true)
      (Audio|SetSoundMixClassOverride "/Game/Sounds/MasterSoundMix.MasterSoundMix" "/Game/Sounds/VolumeSounds.VolumeSounds" _newtrack_0 1.0 0.0 true)
      (Audio|PushSoundMixModifier "/Game/Sounds/MasterSoundMix.MasterSoundMix"))))

(event EventBeginPlay
  (bind _returnvalue (Game|GetPlayerCharacter 0))
  (bind _charactermovement (Variables|/Script/Engine.Character|GetCharacterMovement _returnvalue))
  (bind _returnvalue_2 (UserInterface|CreateWidget "/Game/Blueprints/OutroIntro/IntroWidget.IntroWidget_C" (Game|GetPlayerController 0)))
  (Pawn|Components|CharacterMovement|DisableMovement _charactermovement)
  (CallFunction|SoundFade)
  (UserInterface|Viewport|AddtoViewport _returnvalue_2 0)
  (Default|PlayIntro _returnvalue_2)
  (Utilities|FlowControl|Delay 5.0)
  (Pawn|Components|CharacterMovement|SetMovementMode _charactermovement "MOVE_Walking" 0))

(fn ConstructionScript)