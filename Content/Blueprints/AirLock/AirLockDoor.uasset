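; Airlock door Blueprint that toggles between open and closed when Activate is called, ignoring calls while it is already moving.
; One timeline plays forward or in reverse to slide two door meshes apart or together along local Y.
; A looping-style ambient sound fades in during movement and out on finish, when the Open state flips and fires OnOpen or OnClose.
; BeginPlay sets the timeline time for doors starting open and silences the sound.
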(event EventBeginPlay
  ;[1 1 1] BeginPlay
  (Utilities|FlowControl|Sequence
    (:then_0
      (if (Variables|Default|GetOpen)
        (bind _newtrack_0 (Timeline|Timeline_0 SetNewTime)
          (:Update
            (Transformation|SetRelativeLocation (Variables|Default|Getdoor3) (Math|Vector|Lerp(Vector) "0, 0, 0" "0,-100.000000, 0" _newtrack_0) false false)
            (Transformation|SetRelativeLocation (Variables|Default|Getdoor2) (Math|Vector|Lerp(Vector) "0, 0, 0" "0,100.000000, 0" _newtrack_0) false false))
          (:Finished
            (Variables|Default|SetOpening false)
            (bind _output_get (Variables|Default|SetOpen (not (Variables|Default|GetOpen))))
            (if _output_get
              (Default|CallOnOpen)
              (else
                (Default|CallOnClose)))
            (Audio|Components|Audio|FadeOut (Variables|Default|Get464544__galbenshire__computer-room) 0.5 0.0 "Linear" :!class /Script/Engine.AudioComponent)))))
    (:then_1
      (Audio|Components|Audio|Stop (Variables|Default|Get464544__galbenshire__computer-room)))))

(event EventActivate
  (params (Value :type Integer))
  ;[1 1 1] Activation
  (if (not (Variables|Default|GetOpening))
    (if (Variables|Default|GetOpen)
      (Variables|Default|SetOpening true)
      (Utilities|FlowControl|Sequence
        (:then_0
          (bind _newtrack_0 (Timeline|Timeline_0 Reverse)
            (:Update
              (Transformation|SetRelativeLocation (Variables|Default|Getdoor3) (Math|Vector|Lerp(Vector) "0, 0, 0" "0,-100.000000, 0" _newtrack_0) false false)
              (Transformation|SetRelativeLocation (Variables|Default|Getdoor2) (Math|Vector|Lerp(Vector) "0, 0, 0" "0,100.000000, 0" _newtrack_0) false false))
            (:Finished
              (Variables|Default|SetOpening false)
              (bind _output_get (Variables|Default|SetOpen (not (Variables|Default|GetOpen))))
              (if _output_get
                (Default|CallOnOpen)
                (else
                  (Default|CallOnClose)))
              (Audio|Components|Audio|FadeOut (Variables|Default|Get464544__galbenshire__computer-room) 0.5 0.0 "Linear" :!class /Script/Engine.AudioComponent))))
        (:then_1
          (Audio|Components|Audio|FadeIn (Variables|Default|Get464544__galbenshire__computer-room) 0.2 1.0 0.0 "Linear" :!class /Script/Engine.AudioComponent :!label _label)))
      (else
        (Variables|Default|SetOpening true)
        (Utilities|FlowControl|Sequence
          (:then_0
            (Timeline|Timeline_0 Play))
          (:then_1
            (goto _label)))))))

(fn ConstructionScript)