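; Airlock manager Blueprint that cycles two linked doors, DoorA and DoorB, so one closes before the other opens.
; Activation, ignored while a cycle runs, triggers the lights and, after a delay, toggles the currently open door.
; Door close and open events chain the delayed sequence: the opposite door activates, then lights toggle again and the open-door state flips.
; Button lock, unlock and lights-off functions are empty stubs.
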(event OnClose(DoorA)
  (Utilities|FlowControl|Delay 2.0)
  (if (Variables|Default|GetIsDoorAOpen)
    (Default|Activate (Variables|Default|GetDoorB))
    (else
      (Default|Activate (Variables|Default|GetDoorA)))))

(event OnClose(DoorB)
  (Utilities|FlowControl|Delay 2.0)
  (if (Variables|Default|GetIsDoorAOpen)
    (Default|Activate (Variables|Default|GetDoorB))
    (else
      (Default|Activate (Variables|Default|GetDoorA)))))

(event OnOpen(DoorA)
  (Utilities|FlowControl|Delay 2.0)
  (CallFunction|HandleLights)
  (CallFunction|UnlockButton)
  (Variables|Default|SetIsDoorAOpen (not (Variables|Default|GetIsDoorAOpen)))
  (Variables|Default|SetIsInProgress false))

(event OnOpen(DoorB)
  (Utilities|FlowControl|Delay 2.0)
  (CallFunction|HandleLights)
  (CallFunction|UnlockButton)
  (Variables|Default|SetIsDoorAOpen (not (Variables|Default|GetIsDoorAOpen)))
  (Variables|Default|SetIsInProgress false))

(event EventBeginPlay
  (bind _output_get (Variables|Default|SetIsDoorAOpen (Variables|/Game/Blueprints/AirLock/AirLockDoor.AirLockDoor_C|GetOpen (Variables|Default|GetDoorA))))
  (if _output_get
    _))

(event EventActivate
  (params (Value :type Integer))
  (if (not (Variables|Default|GetIsInProgress))
    (Variables|Default|SetIsInProgress true)
    (CallFunction|HandleLights)
    (CallFunction|LockButton)
    (Utilities|FlowControl|Delay 3.0)
    (if (Variables|Default|GetIsDoorAOpen)
      (Default|Activate (Variables|Default|GetDoorA))
      (else
        (Default|Activate (Variables|Default|GetDoorB))))))

(fn ConstructionScript)

(fn HandleLights
  (for _array_element (Variables|Default|GetLights)
    (Default|Activate _array_element)))

(fn HandleLightsOff)

(fn LockButton)

(fn UnlockButton)