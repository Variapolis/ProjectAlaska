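; Sliding door actor that toggles between open and closed each time its Activate event fires.
; A timeline lerps the Cube along local X, playing forward to open or reversing to close, with a sound on each activation.
; An Opening flag ignores activation mid-movement, and the Open state flips when the timeline finishes.
; If Open is set at BeginPlay, it sets the timeline's time to match the starting state.
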(event EventBeginPlay
  ;[1 1 1] Open
  ;;[1 1 1] BeginPlay
  (if (Variables|Default|GetOpen)
    (bind _newtrack_0 (Timeline|Timeline_0 SetNewTime)
      (:Update
        (Variables|Default|SetOpening true)
        (Transformation|SetRelativeLocation (Variables|Default|GetCube) (Math|Vector|Lerp(Vector) "0, 0, 0" "160.000000,0.000000, 0" _newtrack_0) false false))
      (:Finished
        (Variables|Default|SetOpen (not (Variables|Default|GetOpen)))
        (Variables|Default|SetOpening false)))))

(event EventActivate
  (params (Value :type Integer))
  ;[1 1 1] Open
  ;;[1 1 1] Activation
  (if (not (Variables|Default|GetOpening))
    (Audio|Components|Audio|Play (Variables|Default|GetAudio) 0.0)
    (if (Variables|Default|GetOpen)
      (bind _newtrack_0 (Timeline|Timeline_0 Reverse)
        (:Update
          (Variables|Default|SetOpening true)
          (Transformation|SetRelativeLocation (Variables|Default|GetCube) (Math|Vector|Lerp(Vector) "0, 0, 0" "160.000000,0.000000, 0" _newtrack_0) false false))
        (:Finished
          (Variables|Default|SetOpen (not (Variables|Default|GetOpen)))
          (Variables|Default|SetOpening false)))
      (else
        (Timeline|Timeline_0 Play)))))

(fn ConstructionScript)