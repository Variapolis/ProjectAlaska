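; Alarm lightbar, a child light Blueprint that flashes a spotlight and its bulb mesh while switched on.
; On BeginPlay and on each switch update, it checks IsOn and either plays or stops a flash timeline.
; The timeline scales spotlight intensity from its default and swaps the bulb between alarm and off materials at the curve's midpoint value.
; When off, it passes the spotlight to OffState.
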(event EventBeginPlay
  (|CallParentFunction)
  (if (Variables|Default|GetIsOn)
    (bind _flash (Timeline|Timeline_0 Play)
      (:Update
        (Rendering|Components|Light|SetIntensity (Variables|Default|GetSpotLight) (* _flash (Variables|Default|GetDefaultIntensity)))
        (if (< _flash 0.5)
          (Rendering|Material|SetMaterial (Variables|Default|GetLightBarFlat_LightBar_Bulb) 0 "/Game/Assets/SkirtTrims/LightBar_Bulb_Off.LightBar_Bulb_Off")
          (else
            (Rendering|Material|SetMaterial (Variables|Default|GetLightBarFlat_LightBar_Bulb) 0 "/Game/TwinmotionMaterials/Materials/Emissive/MI_Alarm.MI_Alarm")))))
    (else
      (Utilities|FlowControl|Sequence
        (:then_0
          (Timeline|Timeline_0 Stop))
        (:then_1
          (CallFunction|OffState (Variables|Default|GetSpotLight)))))))

(event Collision|EventActorBeginOverlap
  (params (OtherActor :type Actor%20Object%20Reference))
  (|CallParentFunction OtherActor) ; This node is disabled and will not be called.\nDrag off pins to build functionality.
)

(event EventTick
  (params (DeltaSeconds :type Float%20%28single-precision%29))
  (|CallParentFunction DeltaSeconds) ; This node is disabled and will not be called.\nDrag off pins to build functionality.
)

(event EventEventSwitchUpdate
  (if (Variables|Default|GetIsOn)
    (bind _flash (Timeline|Timeline_0 Play)
      (:Update
        (Rendering|Components|Light|SetIntensity (Variables|Default|GetSpotLight) (* _flash (Variables|Default|GetDefaultIntensity)))
        (if (< _flash 0.5)
          (Rendering|Material|SetMaterial (Variables|Default|GetLightBarFlat_LightBar_Bulb) 0 "/Game/Assets/SkirtTrims/LightBar_Bulb_Off.LightBar_Bulb_Off")
          (else
            (Rendering|Material|SetMaterial (Variables|Default|GetLightBarFlat_LightBar_Bulb) 0 "/Game/TwinmotionMaterials/Materials/Emissive/MI_Alarm.MI_Alarm")))))
    (else
      (Utilities|FlowControl|Sequence
        (:then_0
          (Timeline|Timeline_0 Stop))
        (:then_1
          (CallFunction|OffState (Variables|Default|GetSpotLight)))))))

(fn ConstructionScript
  (|CallParentFunction))