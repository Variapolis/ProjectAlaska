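; Switchable light bar actor with full-power, low-power and off looks, each setting the spotlight's color and intensity plus the bulb mesh material.
; BeginPlay caches the spotlight's intensity and color as the full-power values; low power runs at a tenth of that intensity.
; Activate toggles IsOn, reapplies the matching state and calls the empty SwitchUpdate hook.
; Poweron forces full power regardless of IsOn, while PowerOff re-evaluates state without clearing HasPower.
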(event Custom|Event%20SwitchUpdate)

(event EventBeginPlay
  (bind _spotlight (Variables|Default|GetSpotLight))
  (Variables|Default|SetDefaultIntensity (Variables|/Script/Engine.LightComponentBase|GetIntensity _spotlight))
  (Variables|Default|SetFullPowerColor (Rendering|Components|Light|GetLightColor _spotlight))
  (if (Variables|Default|GetIsOn)
    (if (not (Variables|Default|GetHasPower))
      (CallFunction|LowPowerState _spotlight))
    (else
      (CallFunction|OffState _spotlight))))

(event Collision|EventActorBeginOverlap
  (params (OtherActor :type Actor%20Object%20Reference)))

(event EventTick
  (params (DeltaSeconds :type Float%20%28single-precision%29)))

(event EventPoweron
  (CallFunction|FullPowerState (Variables|Default|GetSpotLight)))

(event EventPowerOff
  (bind _spotlight (Variables|Default|GetSpotLight))
  (if (Variables|Default|GetIsOn)
    (if (not (Variables|Default|GetHasPower))
      (CallFunction|LowPowerState _spotlight))
    (else
      (CallFunction|OffState _spotlight))))

(event EventActivate
  (params (Value :type Integer))
  (Variables|Default|SetIsOn (not (Variables|Default|GetIsOn)))
  (CallFunction|On/OffSwitch)
  (CallFunction|EventSwitchUpdate))

(fn ConstructionScript)

(fn LowPowerState
  (params (Light :type Light%20Component%20Object%20Reference))
  (Rendering|Components|Light|SetLightColor Light (Variables|Default|GetLowPowerColor) true)
  (Rendering|Components|Light|SetIntensity Light (/ (Variables|Default|GetDefaultIntensity) 1e+01))
  (Rendering|Material|SetMaterial (Variables|Default|GetLightBarFlat_LightBar_Bulb) 0 "/Game/TwinmotionMaterials/Materials/Emissive/MI_LowPower.MI_LowPower"))

(fn FullPowerState
  (params (Light :type Light%20Component%20Object%20Reference))
  (Rendering|Components|Light|SetLightColor Light (Variables|Default|GetFullPowerColor) true)
  (Rendering|Components|Light|SetIntensity Light (Variables|Default|GetDefaultIntensity))
  (Variables|Default|SetHasPower true)
  (Rendering|Material|SetMaterial (Variables|Default|GetLightBarFlat_LightBar_Bulb) 0 "/Game/TwinmotionMaterials/Materials/Emissive/MI_FullPower.MI_FullPower"))

(fn OffState
  (params (Light :type Light%20Component%20Object%20Reference))
  (Rendering|Components|Light|SetLightColor Light (Variables|Default|GetOffColor) true)
  (Rendering|Components|Light|SetIntensity Light 0.0)
  (Rendering|Material|SetMaterial (Variables|Default|GetLightBarFlat_LightBar_Bulb) 0 "/Game/Assets/SkirtTrims/LightBar_Bulb_Off.LightBar_Bulb_Off"))

(fn On/OffSwitch
  (bind _spotlight (Variables|Default|GetSpotLight))
  (if (Variables|Default|GetIsOn)
    (if (Variables|Default|GetHasPower)
      (CallFunction|FullPowerState _spotlight)
      (else
        (CallFunction|LowPowerState _spotlight)))
    (else
      (CallFunction|OffState _spotlight))))